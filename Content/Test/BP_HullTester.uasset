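; BP_HullTester is a test actor that exercises the hardpoint and stat functions of an MCPHull component on a referenced hull actor.
; On BeginPlay it fetches that component, then after timed delays adds an extra hardpoint, removes it again and overrides the hull's base Weight stat.
; The sequence runs once, with no checks or reporting of results.
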(event EventBeginPlay
  (bind _mcphardpoint1 (Variables|Default|GetMCPHardpoint1))
  (Variables|Default|SetHull (Actor|GetComponentbyClass (Variables|Default|GetHullActor) "/Script/ComplexGameSystems.MCPHull"))
  (Utilities|FlowControl|Delay 1e+01)
  ;[1 1 1] Add and Remove
  (Class|MCPHull|AddExtraHardpoint (Variables|Default|GetHull) _mcphardpoint1)
  (Utilities|FlowControl|Delay 1.0)
  (Class|MCPHull|RemoveExtraHardpoint (Variables|Default|GetHull) _mcphardpoint1)
  (Utilities|FlowControl|Delay 1.0)
  (Class|MCPHull|SetBaseStatValue (Variables|Default|GetHull) "Weight" 3.0))

(event Collision|EventActorBeginOverlap
  (params (OtherActor :type Actor%20Object%20Reference)))

(event EventTick
  (params (DeltaSeconds :type Float%20%28single-precision%29)))

(fn ConstructionScript)